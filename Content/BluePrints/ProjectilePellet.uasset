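; ProjectilePellet is a pellet projectile Blueprint that launches itself forward when spawned and removes itself after a set lifetime.
; On BeginPlay it applies a single large, mass-dependent force to BulletMesh along the actor's forward vector, leaving its flight to physics.
; Tick accumulates elapsed time and destroys the actor once it reaches MaxTime.
; The graphs contain no hit or damage logic.
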(event `self.ReceiveBeginPlay`
  (`PrimitiveComponent.AddForce` (`self.BulletMesh`) (* (`self.GetActorForwardVector`) 600000.0) "None" false))

(event `self.ReceiveTick`
  (params (DeltaSeconds :type "Float (single-precision)"))
  (set `self.timer` (+ DeltaSeconds (`self.timer`)))
  (if (>= (`self.timer`) (`self.maxTime`))
    (`self.K2_DestroyActor`)))

(fn `UserConstructionScript`)